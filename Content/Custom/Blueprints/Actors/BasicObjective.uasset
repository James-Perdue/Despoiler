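; BasicObjective is an actor that registers itself as the objective of the Attacker team in the Despoiler game mode.
; A short one-shot timer started on BeginPlay calls SetObjective.
; That function casts the game mode to DespoilerGameMode, looks up Attacker in its Teams map and, if that team is valid, passes itself to the team's own SetObjective.
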(event `self.ReceiveBeginPlay`
  (`KismetSystemLibrary.K2_SetTimerDelegate` (delegate `CustomEvent`) 0.5))

(event `CustomEvent`
  (`self.SetObjective`))

(fn `SetObjective`
  (bind _asdespoiler_game_mode (cast `DespoilerGameMode` (`GameplayStatics.GetGameMode`)))
  (bind (_value _returnvalue) (`BlueprintMapLibrary.Map_Find` (`DespoilerGameMode.Teams` _asdespoiler_game_mode) "Attacker"))
  (if _returnvalue
    (`/Engine/EditorBlueprintResources/StandardMacros.IsValid` _value
      (:`Is Valid`
        (`Team.SetObjective` _value self)))))

(fn `UserConstructionScript`)