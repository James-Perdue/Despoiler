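; Player pawn Blueprint that lets the user toggle control between itself and a spectator camera.
; On BeginPlay it adds the live session Enhanced Input mapping context and spawns the spectator camera at its own transform.
; The swap-camera input action drives a FlipFlop that makes the first player controller alternately possess the spectator camera and this pawn.
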(event `self.ReceiveBeginPlay`
  (bind _asplayer_controller (cast `/Game/Custom/Blueprints/Controller/PlayerController` (`GameplayStatics.GetPlayerController` 0)))
  (`EnhancedInputSubsystemInterface.AddMappingContext` (pcsubsystem `EnhancedInputLocalPlayerSubsystem` _asplayer_controller) "/Game/Custom/Blueprints/Controller/LiveSessionMapping.LiveSessionMapping" 0 (struct))
  (bind _returnvalue (`|SpawnActorFromClass` "/Game/Custom/Blueprints/Controller/SpectatorCam.SpectatorCam_C" (`self.GetTransform`) "Undefined" "MultiplyWithRoot" null null)))

(event `EnhancedInput|/Game/Custom/Blueprints/Controller/IA_SwapCamera`
  (params (ActionValue :type Boolean) (ElapsedSeconds :type "Float (double-precision)") (TriggeredSeconds :type "Float (double-precision)") (InputAction :type "InputAction Object Reference" :default "/Game/Custom/Blueprints/Controller/IA_SwapCamera.IA_SwapCamera"))
  (bind _returnvalue (`GameplayStatics.GetPlayerController` 0))
  (:`Triggered`
    (`/Engine/EditorBlueprintResources/StandardMacros.FlipFlop`
      (:`A`
        (`Controller.Possess` _returnvalue (stale `self.ReceiveBeginPlay` _returnvalue)))
      (:`B`
        (`Controller.Possess` _returnvalue self)))))

(fn `UserConstructionScript`)