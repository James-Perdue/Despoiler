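; SpectatorCam is a spectator camera Blueprint that handles pausing and switching back to the player.
; The pause input uses a FlipFlop to create and show a pause menu with the cursor and game pause, then remove it and resume.
; The swap camera input finds the Player and PlayerCamera actors, possesses the Player, and sets the view target to the PlayerCamera.
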(event `self.ReceiveBeginPlay`)

(event `EnhancedInput|/Game/Custom/Blueprints/Controller/IA_Pause`
  (params (ActionValue :type Boolean) (ElapsedSeconds :type "Float (double-precision)") (TriggeredSeconds :type "Float (double-precision)") (InputAction :type "InputAction Object Reference" :default "/Game/Custom/Blueprints/Controller/IA_Pause.IA_Pause"))
  (bind _returnvalue (`GameplayStatics.GetPlayerController` 0))
  (bind _pause_menu_ui (`self.Pause Menu UI`))
  (:`Triggered`
    (`/Engine/EditorBlueprintResources/StandardMacros.FlipFlop`
      (:`A`
        (bind _returnvalue_2 (`|CreateWidget` "/Game/Custom/Blueprints/UI/PauseMenuUI.PauseMenuUI_C" _returnvalue))
        (bind _output_get (set `self.Pause Menu UI` _returnvalue_2))
        (`UserWidget.AddToViewport` _output_get 0)
        (`GameplayStatics.SetGamePaused` true)
        (set `PlayerController.bShowMouseCursor` true _returnvalue))
      (:`B`
        (`/Engine/EditorBlueprintResources/StandardMacros.IsValid` _pause_menu_ui
          (:`Is Valid`
            (`Widget.RemoveFromParent` _pause_menu_ui)
            (set `PlayerController.bShowMouseCursor` false _returnvalue)
            (`GameplayStatics.SetGamePaused` false)))))))

(event `EnhancedInput|/Game/Custom/Blueprints/Controller/IA_SwapCamera`
  (params (ActionValue :type Boolean) (ElapsedSeconds :type "Float (double-precision)") (TriggeredSeconds :type "Float (double-precision)") (InputAction :type "InputAction Object Reference" :default "/Game/Custom/Blueprints/Controller/IA_SwapCamera.IA_SwapCamera"))
  (bind _returnvalue (`GameplayStatics.GetPlayerController` 0))
  (:`Triggered`
    (bind _returnvalue_2 (`GameplayStatics.GetActorOfClass` "/Game/Custom/Blueprints/Controller/PlayerCamera.PlayerCamera_C"))
    (bind _returnvalue_3 (`GameplayStatics.GetActorOfClass` "/Game/Custom/Blueprints/Controller/Player.Player_C"))
    (`Controller.Possess` _returnvalue _returnvalue_3)
    (`PlayerController.SetViewTargetWithBlend` _returnvalue _returnvalue_2 0.0 "VTBlend_Linear" 0.0 false)))

(fn `UserConstructionScript`)